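; BP_Page is an interactable collectible page that the player picks up to count down the pages remaining.
; On BeginPlay it applies one of eight page materials at random to its plane mesh.
; On interact it plays a collect sound, decrements PagesLeft on the game mode through the player's reference, then destroys itself.
; The check for zero pages left has nothing wired to either branch.
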(event EventBeginPlay
  (Variables|Default|SetPageIndex (Math|Random|RandomIntegerinRange 0 7))
  (Rendering|Material|SetMaterial (Variables|Default|GetPlane) 0 (Utilities|Select :Index (Variables|Default|GetPageIndex) :Option%200 "/Game/_Main/Pages/1_Mat.1_Mat" :Option%201 "/Game/_Main/Pages/2_Mat.2_Mat" :Option%202 "/Game/_Main/Pages/3_Mat.3_Mat" :Option%203 "/Game/_Main/Pages/4_Mat.4_Mat" :Option%204 "/Game/_Main/Pages/5_Mat.5_Mat" :Option%205 "/Game/_Main/Pages/6_Mat.6_Mat" :Option%206 "/Game/_Main/Pages/7_Mat.7_Mat" :Option%207 "/Game/_Main/Pages/8_Mat.8_Mat")))

(event EventOnInteract
  (params (Player :type BP%20Player%20Object%20Reference))
  (Variables|Default|SetPlayerRef Player)
  (Audio|PlaySound2D "/Game/_Main/SFX/Paper/CollectPage.CollectPage" 1.0 1.0 0.0 0 0)
  (bind _result (Math|Integer|DecrementInt (Variables|/Game/_Main/Framework/BP_GameMode.BP_GameMode_C|GetPagesLeft (Variables|/Game/_Main/_Player/BP_Player.BP_Player_C|GetGameModeRef (Variables|Default|GetPlayerRef))))
    (:%20%20
      (bind _output_get (Variables|/Game/_Main/Framework/BP_GameMode.BP_GameMode_C|SetPagesLeft (Variables|/Game/_Main/_Player/BP_Player.BP_Player_C|GetGameModeRef (Variables|Default|GetPlayerRef)) _result))
      (if (== _output_get 0)
        _
        (else
          _))
      (Actor|DestroyActor))))

(fn ConstructionScript)