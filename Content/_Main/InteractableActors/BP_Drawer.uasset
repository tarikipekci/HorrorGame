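; BP_Drawer is an interactable drawer that slides open and closed when the player interacts with it.
; OnInteract uses a FlipFlop to alternate between playing and reversing a timeline that lerps the mesh's relative Y position, with an open or close sound at the mesh.
; The construction script shows or hides the Key component based on the HasKey flag.
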(event EventOnInteract
  (params (Player :type BP%20Player%20Object%20Reference))
  (bind _drawermesh (Variables|Default|GetDrawerMesh))
  (bind _returnvalue (Transformation|GetWorldLocation _drawermesh))
  (Utilities|FlowControl|FlipFlop
    (:A
      (Audio|PlaySoundatLocation "/Game/_Main/SFX/Drawer/DrawerOpen.DrawerOpen" _returnvalue "0, 0, 0" 1.0 1.0 0.0 0 0 0 0)
      (bind _alpha (Timeline|TL_OpenDrawer Play)
        (:Update
          (Transformation|SetRelativeLocation (Variables|Default|GetDrawerMesh) (Math|Vector|MakeVector 0.0 (Math|Float|Lerp 0.0 4e+01 _alpha) 0.0) false false))))
    (:B
      (Audio|PlaySoundatLocation "/Game/_Main/SFX/Drawer/DrawerClose.DrawerClose" _returnvalue "0, 0, 0" 1.0 1.0 0.0 0 0 0 0)
      (Timeline|TL_OpenDrawer Reverse))))

(fn ConstructionScript
  (bind _key (Variables|Default|GetKey))
  (if (Variables|Default|GetHasKey)
    (Rendering|SetVisibility _key true false)
    (else
      (Rendering|SetVisibility _key false false))))