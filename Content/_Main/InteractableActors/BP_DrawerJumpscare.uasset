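; Interactable drawer that springs a one-time spider monster jumpscare on the player when first opened.
; OnInteract toggles open and close through a FlipFlop, playing a sound and sliding the mesh on a timeline that is not retriggered mid-scare.
; Opening fires a DoOnce Jumpscare: the spider plays a scream animation, lunges at the player camera via timeline lerp and look-at rotation, then its component is destroyed.
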(event Custom|Jumpscare
  (bind _playerref (Variables|Default|GetPlayerRef))
  (bind _spidermonster (Variables|Default|GetSpiderMonster))
  (bind _spidermonster_2 (Variables|Default|GetSpiderMonster))
  (bind _spidermonster_3 (Variables|Default|GetSpiderMonster))
  (bind _returnvalue (Transformation|GetWorldLocation _spidermonster))
  (bind _camera (Variables|/Game/_Main/_Player/BP_Player.BP_Player_C|GetCamera _playerref))
  (bind _returnvalue_2 (Transformation|GetWorldLocation _camera))
  (bind _returnvalue_3 (+ _returnvalue_2 "4.000000,0.000000,0.000000"))
  (bind _returnvalue_4 (Math|Rotator|FindLookatRotation _returnvalue _returnvalue_3))
  (Utilities|FlowControl|DoOnce false
    (:Completed
      (Variables|Default|SetIsJumpscarePlaying? true)
      (Components|Animation|PlayAnimation (Variables|Default|GetSpiderMonster) "/Game/_Main/3dModels/SpiderMonster/source/SpiderMonsterscreem/SkeletalMeshes/SpiderMonsterscreem_Anim.SpiderMonsterscreem_Anim" false)
      (Utilities|FlowControl|Delay 0.3)
      (Audio|PlaySound2D "/Game/_Main/SFX/Jumpscares/SpiderMonsterJumpscare.SpiderMonsterJumpscare" 0.05 1.0 0.0 0 0)
      (Utilities|FlowControl|Sequence
        (:then_0
          (bind _alpha (Timeline|TL_Jumpscare Play)
            (:Update
              (Utilities|IsValid _spidermonster_2
                (:Is%20Valid
                  (Transformation|SetWorldLocation _spidermonster_2 (Math|Vector|Lerp(Vector) _returnvalue _returnvalue_3 _alpha) false false)
                  (Transformation|SetWorldRotation _spidermonster_2 (Math|Rotator|MakeRotator (.roll _returnvalue_4) 0.0 (- (.yaw _returnvalue_4) 8e+01)) false false))))))
        (:then_1
          (Utilities|FlowControl|Delay 0.35)
          (Variables|Default|SetIsJumpscarePlaying? false)
          (Audio|Components|Audio|Stop _spidermonster_3)
          (Components|DestroyComponent _spidermonster_3))))))

(event EventOnInteract
  (params (Player :type BP%20Player%20Object%20Reference))
  (bind _drawermesh (Variables|Default|GetDrawerMesh))
  (bind _isjumpscareplaying_ (Variables|Default|GetIsJumpscarePlaying?))
  (bind _spidermonster (Variables|Default|GetSpiderMonster))
  (bind _returnvalue (Transformation|GetWorldLocation _drawermesh))
  (bind _returnvalue_2 (not _isjumpscareplaying_))
  (Variables|Default|SetPlayerRef Player)
  (Utilities|FlowControl|FlipFlop
    (:A
      (Utilities|FlowControl|Sequence
        (:then_0
          (Audio|PlaySoundatLocation "/Game/_Main/SFX/Drawer/DrawerOpen.DrawerOpen" _returnvalue "0, 0, 0" 1.0 1.0 0.0 0 0 0 0)
          (if _returnvalue_2
            (bind _alpha (Timeline|TL_OpenDrawer Play)
              (:Update
                (Transformation|SetRelativeLocation (Variables|Default|GetDrawerMesh) (Math|Vector|MakeVector 0.0 (Math|Float|Lerp 0.0 4e+01 _alpha) 0.0) false false)
                (Utilities|IsValid (Variables|Default|GetSpiderMonster)
                  (:Is%20Valid
                    (Transformation|SetWorldRotation _spidermonster (Math|Rotator|MakeRotator 0.0 0.0 (.yaw (Math|Rotator|FindLookatRotation (Transformation|GetWorldLocation _spidermonster) (+ (Transformation|GetWorldLocation (Variables|/Game/_Main/_Player/BP_Player.BP_Player_C|GetCamera (Variables|Default|GetPlayerRef))) "7.000000,0.000000,0.000000")))) false false)))))))
        (:then_1
          (CallFunction|Jumpscare))))
    (:B
      (Audio|PlaySoundatLocation "/Game/_Main/SFX/Drawer/DrawerClose.DrawerClose" _returnvalue "0, 0, 0" 1.0 1.0 0.0 0 0 0 0)
      (if _returnvalue_2
        (Timeline|TL_OpenDrawer Reverse)))))

(fn ConstructionScript)