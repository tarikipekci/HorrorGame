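; Interactable door with a configurable mesh that the player opens and closes, with optional key-based locking.
; While locked, it plays a locked sound if the Key reference is still valid; otherwise a gate lets the unlock sound play once before a short delay clears the lock.
; A timeline swings the mesh open away from the player, using a dot product to pick the direction, and reverses to close.
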(event Custom|Open/Close%20Door
  (bind _self self)
  (bind _staticmesh (Variables|Default|GetStaticMesh))
  (bind _returnvalue (Transformation|GetWorldLocation _staticmesh))
  ;[0.15 0.15 0.15 0.5] Calculate Dot Product
  (if (Variables|Default|GetClosed?)
    (Variables|Default|SetClosed? false)
    (Audio|PlaySoundatLocation "/Game/_Main/SFX/Door/DoorOpen.DoorOpen" _returnvalue "0, 0, 0" 1.0 1.0 0.0 0 0 0 0)
    (Variables|Default|SetDotProduct (Math|Vector|DotProduct (Math|Vector|Normalize (- (Transformation|GetActorLocation _self) (Transformation|GetActorLocation (Variables|Default|GetPlayerRef)))) (Transformation|GetActorForwardVector _self)))
    (bind _alpha (Timeline|TL_OpenDoor Play)
      (:Update
        (Transformation|SetRelativeRotation (Variables|Default|GetStaticMesh) (Math|Rotator|Lerp(Rotator) "0, 0, 0" (Math|Rotator|MakeRotator 0.0 0.0 (* (Variables|Default|GetOpenAngle) (Math|Float|SelectFloat 1.0 -1.0 (>= (Variables|Default|GetDotProduct) 0.0)))) _alpha) false false)))
    (else
      (Variables|Default|SetClosed? true)
      (Audio|PlaySoundatLocation "/Game/_Main/SFX/Door/DoorClose.DoorClose" _returnvalue "0, 0, 0" 1.0 1.0 0.0 0 0 0 0)
      (Timeline|TL_OpenDoor Reverse))))

(event EventOnInteract
  (params (Player :type BP%20Player%20Object%20Reference))
  (bind _staticmesh (Variables|Default|GetStaticMesh))
  (bind _returnvalue (Transformation|GetWorldLocation _staticmesh))
  (Variables|Default|SetPlayerRef Player)
  (if (Variables|Default|GetLocked?)
    (Utilities|IsValid (Variables|Default|GetKey)
      (:Is%20Valid
        (Audio|PlaySoundatLocation "/Game/_Main/SFX/Door/DoorsLocked.DoorsLocked" _returnvalue "0, 0, 0" 1.0 1.0 0.0 0 0 0 0))
      (:Is%20Not%20Valid
        (Utilities|FlowControl|Gate false :!label _label
          (:Exit
            (Audio|PlaySoundatLocation "/Game/_Main/SFX/Door/Door_Unlocking.Door_Unlocking" _returnvalue "0, 0, 0" 1.0 1.0 0.0 0 0 0 0)
            (Utilities|FlowControl|Sequence
              (:then_0
                (Utilities|FlowControl|Delay 1.3)
                (Variables|Default|SetLocked? false))
              (:then_1
                (goto _label Close)))))))
    (else
      (CallFunction|Open/CloseDoor))))

(fn ConstructionScript
  (Components|StaticMesh|SetStaticMesh (Variables|Default|GetStaticMesh) (Variables|Default|GetDoorMesh)))