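; BP_LightSwitch is an interactable wall switch that toggles linked lights, or only clicks when it is not working.
; On interact, it inverts each linked light's visibility individually, playing a sound and setting the switch transform per light.
; The last light's resulting state sets IsLightOn, which selects the on or off material for linked lamp meshes.
; When not working, a FlipFlop alternates the switch pose and flashlight sounds without affecting lights.
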(event EventOnInteract
  (params (Player :type BP%20Player%20Object%20Reference))
  (bind _switch (Variables|Default|GetSwitch))
  (bind _switch_2 (Variables|Default|GetSwitch))
  (bind _returnvalue (Transformation|GetWorldLocation _switch_2))
  (if (Variables|Default|GetIsWorking?)
    (Utilities|FlowControl|Sequence
      (:then_0
        (for _array_element (Variables|Default|GetLightsToToggle)
          (if (Rendering|IsVisible (Variables|/Script/Engine.Light|GetLightComponent _array_element))
            (Variables|Default|SetIsLightOn? false)
            (Audio|PlaySoundatLocation "/Game/_Main/SFX/LightSwitch/LightOff.LightOff" (Transformation|GetWorldLocation (Variables|Default|GetSwitch)) "0, 0, 0" 1.0 1.0 0.0 0 0 0 0)
            (Rendering|SetVisibility (Variables|/Script/Engine.Light|GetLightComponent _array_element) false false)
            (Transformation|SetRelativeTransform _switch (Math|Transform|MakeTransform "0, 0, 0" "0, 0, 0" "1.000000,1.000000,1.000000") false false)
            (else
              (Variables|Default|SetIsLightOn? true)
              (Audio|PlaySoundatLocation "/Game/_Main/SFX/LightSwitch/LightOn.LightOn" (Transformation|GetWorldLocation (Variables|Default|GetSwitch)) "0, 0, 0" 1.0 1.0 0.0 0 0 0 0)
              (Rendering|SetVisibility (Variables|/Script/Engine.Light|GetLightComponent _array_element) true false)
              (Transformation|SetRelativeTransform _switch (Math|Transform|MakeTransform "0.000000,-5.000000,4.000000" "0.000000,0.000000,60.000000") false false)))))
      (:then_1
        (for _array_element_2 (Variables|Default|GetLampBPs)
          (if (Variables|Default|GetIsWorking?)
            (Rendering|Material|SetMaterial (Variables|/Game/_Main/InteractableActors/BP_Lamp.BP_Lamp_C|GetLampMesh _array_element_2) (Variables|/Game/_Main/InteractableActors/BP_Lamp.BP_Lamp_C|GetLightMaterialSlot _array_element_2) (select (Variables|Default|GetIsLightOn?) "/Game/_Main/3dModels/HangingLight/LightOn.LightOn" "/Game/_Main/3dModels/HangingLight/LightOff.LightOff"))))))
    (else
      (Utilities|FlowControl|FlipFlop
        (:A
          (Transformation|SetRelativeTransform _switch_2 (Math|Transform|MakeTransform "0.000000,-5.000000,4.000000" "0.000000,0.000000,60.000000") false false)
          (Audio|PlaySoundatLocation "/Game/_Main/SFX/Flashlight/FlashlightOn.FlashlightOn" _returnvalue "0, 0, 0" 1.0 1.0 0.0 0 0 0 0))
        (:B
          (Transformation|SetRelativeTransform _switch_2 (Math|Transform|MakeTransform "0, 0, 0" "0, 0, 0" "1.000000,1.000000,1.000000") false false)
          (Audio|PlaySoundatLocation "/Game/_Main/SFX/Flashlight/FlashlightOff.FlashlightOff" _returnvalue "0, 0, 0" 1.0 1.0 0.0 0 0 0 0))))))

(fn ConstructionScript)