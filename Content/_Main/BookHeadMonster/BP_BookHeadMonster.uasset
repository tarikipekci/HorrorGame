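; BP_BookHeadMonster is a roaming monster AI that hunts the player and ends the chase with a jumpscare.
; It wanders to random reachable points, while PawnSensing sends it to heard noises or into a faster chase that reverts to roaming via a retriggerable delay.
; Reaching the player triggers a one-time cutscene that disables input, turns the camera toward the monster, and uses montage notifies to release it and break the flashlight.
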(event OnSeePawn(PawnSensing)
  (params (Pawn :type Pawn%20Object%20Reference))
  ;[0.15 0.15 0.15 0.5] Chase Player
  (Utilities|FlowControl|Sequence
    (:then_0
      (Variables|/Script/Engine.CharacterMovementComponent|SetMaxWalkSpeed (Variables|Character|GetCharacterMovement) (Variables|Default|GetChasingSpeed))
      (AI|AIMoveTo self "0, 0, 0" Pawn 1.5e+02 false
        (:OnSuccess
          (Utilities|FlowControl|DoOnce false
            (:Completed
              (CallFunction|Jumpscare))))))
    (:then_1
      (Utilities|FlowControl|RetriggerableDelay 1.0)
      (Variables|/Script/Engine.CharacterMovementComponent|SetMaxWalkSpeed (Variables|Character|GetCharacterMovement) (Variables|Default|GetDefaultSpeed))
      (CallFunction|RandomRoam))))

(event OnHearNoise(PawnSensing)
  (params (Instigator :type Pawn%20Object%20Reference) (Location :type Vector%20%28by%20ref%29 :default "0, 0, 0") (Volume :type Float%20%28single-precision%29))
  ;[0.15 0.15 0.15 0.5] AI Hearing
  (AI|AIMoveTo self Location 0 5.0 false))

(event Custom|RandomRoam
  ;[0.15 0.15 0.15 0.5] Random Roam
  (AI|AIMoveTo self (.RandomLocation (AI|Navigation|GetRandomReachablePointinRadius (Transformation|GetActorLocation) 3e+03 0 0)) 0 5.0 false
    (:OnSuccess
      _)
    (:OnFail
      _))
  (Utilities|FlowControl|Delay 3.0)
  (CallFunction|RandomRoam))

(event Custom|Jumpscare
  (bind _playerref (Variables|Default|GetPlayerRef))
  (bind _spotlight (Variables|/Game/_Main/_Player/BP_Player.BP_Player_C|GetSpotLight _playerref))
  ;[0.15 0.15 0.15 0.5] Jumpscare cutscene
  (Transformation|SetActorRotation (Math|Rotator|FindLookatRotation (Transformation|GetActorLocation) (Transformation|GetActorLocation (Variables|Default|GetPlayerRef))))
  (Pawn|Components|CharacterMovement|DisableMovement (Variables|Character|GetCharacterMovement))
  (Input|DisableInput (Variables|Default|GetPlayerRef) (Game|GetPlayerController 0))
  (Variables|Default|SetLockCamera? true)
  (bind _notifyname (Animation|Montage|PlayMontage (Variables|Character|GetMesh) "/Game/_Main/BookHeadMonster/Animations/MutantSwiping_UE_Montage.MutantSwiping_UE_Montage")
    (:then
      (Audio|PlaySound2D "/Game/_Main/SFX/BookHeadMonster/BookHeadMonster.BookHeadMonster" 1.0 1.0 0.0 0 0)
      (Camera|SetFieldOfView (Variables|/Game/_Main/_Player/BP_Player.BP_Player_C|GetCamera _playerref) 1.2e+02)
      (Rendering|Lighting|SetOuterConeAngle _spotlight 6e+01)
      (if (not (Rendering|IsVisible _spotlight))
        (Rendering|SetVisibility _spotlight true false)
        (Audio|PlaySound2D "/Game/_Main/SFX/Flashlight/FlashlightOn.FlashlightOn" 1.0 1.0 0.0 0 0)))
    (:OnNotifyBegin
      (if (== _notifyname "StopCamera")
        (Variables|Default|SetLockCamera? false)
        (elif (== _notifyname "BreakFlashlight")
          (Audio|PlaySound2D "/Game/_Main/SFX/Bulb/BulbBreak.BulbBreak" 1.0 1.0 0.0 0 0)
          (Rendering|SetVisibility (Variables|/Game/_Main/_Player/BP_Player.BP_Player_C|GetSpotLight (Variables|Default|GetPlayerRef)) false false)
          (Audio|PlaySound2D "/Game/_Main/SFX/BookHeadMonster/Hit.Hit" 1.0 1.0 0.0 0 0))))))

(event EventBeginPlay
  ;[0.15 0.15 0.15 0.5] Begin Play
  (Utilities|FlowControl|Sequence
    (:then_0
      (bind _asbp_player (Utilities|Casting|CastToBP_Player (Game|GetPlayerCharacter 0)))
      (Variables|Default|SetPlayerRef _asbp_player))
    (:then_1
      (CallFunction|RandomRoam))))

(event EventTick
  (params (DeltaSeconds :type Float%20%28single-precision%29))
  ;[0.15 0.15 0.15 0.5] Tick
  (if (Variables|Default|GetLockCamera?)
    (Pawn|SetControlRotation (Game|GetPlayerController 0) (Math|Interpolation|RInterpTo (Pawn|GetControlRotation (Variables|Default|GetPlayerRef) :!class /Script/Engine.Pawn) (Math|Rotator|FindLookatRotation (Transformation|GetWorldLocation (Variables|/Game/_Main/_Player/BP_Player.BP_Player_C|GetCamera (Variables|Default|GetPlayerRef))) (Transformation|GetSocketLocation (Variables|Character|GetMesh) "lowerarm_l")) (Utilities|Time|GetWorldDeltaSeconds) 1e+01))))

(fn ConstructionScript)